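; Main menu game mode that restores the saved weapon selection when play begins.
; If a "save1" save exists, it loads it as a ShooterSaveGame and copies the saved weapon ID into the MyGameSettings game instance.
; It then has the game instance initialize its weapon list.
; A node copying the saved level is left disconnected, so level is not restored here.
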(event EventBeginPlay
  (bind _returnvalue (SaveGame|DoesSaveGameExist "save1"))
  (if _returnvalue
    (bind _returnvalue_2 (SaveGame|LoadGamefromSlot "save1"))
    (bind _asshooter_save_game (Utilities|Casting|CastToShooterSaveGame _returnvalue_2))
    (bind _asmy_game_settings (Utilities|Casting|CastToMyGameSettings (Game|GetGameInstance)))
    (Variables|/Game/BluePrints/MyGameSettings.MyGameSettings_C|SetIDCurrentWeapon _asmy_game_settings (Variables|/Game/BluePrints/ShooterSaveGame.ShooterSaveGame_C|GetIdWeaponFromSaveGame _asshooter_save_game))
    (Default|IniTWeaponList _asmy_game_settings)))

(event EventTick
  (params (DeltaSeconds :type Float%20%28single-precision%29)))

(fn ConstructionScript)