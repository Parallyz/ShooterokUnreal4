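; Player character Blueprint for a first-person shooter, handling firing, reloading, sprinting, damage, pause, game over and save/load input.
; BeginPlay creates the HUD and applies the Game Instance's weapon ID, which InitWeapon maps to gun meshes.
; Sprint stamina drains and refills through self-calling events with short Delays.
; Enemy projectile overlaps deal damage and end the game at zero health, while Tick emits zero-loudness pawn noise.
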(event OnComponentBeginOverlap(CapsuleComponent)
  (params (OverlappedComponent :type Primitive%20Component%20Object%20Reference) (OtherActor :type Actor%20Object%20Reference) (OtherComp :type Primitive%20Component%20Object%20Reference) (OtherBodyIndex :type Integer) (bFromSweep :type Boolean) (SweepResult :type Hit%20Result%20Structure%20%28by%20ref%29))
  ;[1 1 1] GetDamage
  (bind _asfpsprojectile (Utilities|Casting|CastToFPSProjectile OtherActor))
  (bind _asmy_enemy_bp (Utilities|Casting|CastToMyEnemyBP (Components|GetOwner _asfpsprojectile)))
  (bind _asmy_character_bp (Utilities|Casting|CastToMyCharacterBP (Game|GetPlayerCharacter 0)))
  (Class|MyCharacter|DealDamage _asmy_character_bp (Math|Conversions|ToFloat(Integer) (Variables|/Script/Shooterok.Enemy|GetdamageFromBullets _asmy_enemy_bp)))
  (Audio|PlaySoundatLocation "/Game/Sounds/bullet_hit_body_Cue.bullet_hit_body_Cue" (Transformation|GetActorLocation) "0, 0, 0" 1.0 1.0 0.0 0 0 0)
  (if (<= (Variables|Default|GetHealth) 0.0)
    (CallFunction|EndGame)))

(event Custom|DrainStamina
  ;[1 1 1] Run with Stamina
  (if (Variables|Default|GetRunning)
    (bind _output_get (Variables|Default|SetStamina (Math|Float|Clamp(Float) (- (Variables|Default|GetStamina) 1.0) 0.0 (Variables|Default|GetFullStamina))))
    (if (== _output_get 0.0)
      (Variables|Default|SetRunning false)
      (Variables|/Script/Engine.CharacterMovementComponent|SetMaxWalkSpeed (Variables|Character|GetCharacterMovement) 6e+02)
      (else
        (Utilities|FlowControl|Delay 0.01)
        (CallFunction|DrainStamina)))))

(event Custom|RefreshStamin
  ;[1 1 1] Refresh Stamina
  (if (not (Variables|Default|GetRunning))
    (if (not (== (Variables|Default|GetStamina) (Variables|Default|GetFullStamina)))
      (Variables|Default|SetStamina (Math|Float|Clamp(Float) (+ (Variables|Default|GetStamina) 1.0) 0.0 (Variables|Default|GetFullStamina)))
      (Utilities|FlowControl|Delay 0.01)
      (CallFunction|RefreshStamin))))

(event Custom|EndGame
  (bind _returnvalue (Game|GetPlayerController 0))
  ;[1 1 1] Game over
  (Utilities|IsValid (Variables|Default|GetPause%20Menu%20Reference)
    (:Is%20Valid
      _)
    (:Is%20Not%20Valid
      (bind _returnvalue_2 (UserInterface|CreateWidget "/Game/BluePrints/Widgets/GameOverWidget.GameOverWidget_C"))))
  (Variables|/Script/Engine.PlayerController|SetbShowMouseCursor _returnvalue true)
  (Input|SetInputModeUIOnly _returnvalue _returnvalue_2 "DoNotLock")
  (UserInterface|Viewport|AddtoViewport _returnvalue_2 0)
  (Game|SetGamePaused true))

(event EventBeginPlay
  ;[1 1 1] Load Config
  (Utilities|FlowControl|Sequence
    (:then_0
      (bind _returnvalue (UserInterface|CreateWidget "/Game/BluePrints/Widgets/User_UI.User_UI_C"))
      (bind _output_get (Variables|Default|SetHud%20ref _returnvalue))
      (UserInterface|Viewport|AddtoViewport _output_get 0)
      (Input|SetInputModeGameOnly (Game|GetPlayerController 0)))
    (:then_1
      (bind _asmy_game_settings (Utilities|Casting|CastToMyGameSettings (Game|GetGameInstance)))
      (Utilities|FlowControl|Sequence
        (:then_1
          (bind _asmy_character_bp (Utilities|Casting|CastToMyCharacterBP (Game|GetPlayerCharacter 0)))
          (Class|MyCharacter|SetBaseUpRate _asmy_character_bp 45.0)
          (Class|MyCharacter|SetBaseTurnRate _asmy_character_bp 45.0)
          (Class|MyCharacter|InitWeaponbyId _asmy_character_bp (Variables|/Game/BluePrints/MyGameSettings.MyGameSettings_C|GetIDCurrentWeapon _asmy_game_settings))
          (CallFunction|InitWeapon))))))

(event EventTick
  (params (DeltaSeconds :type Float%20%28single-precision%29))
  (bind _returnvalue (Game|GetPlayerCharacter 0))
  ;[1 1 1] Make noise
  (Class|PawnNoiseEmitterComponent|MakeNoise (Variables|Default|GetPawnNoiseEmitter) _returnvalue 0.0 (Transformation|GetActorLocation _returnvalue)))

(event Input|ActionEvents|InputActionRun
  (params (Key :type Key%20Structure :default "None"))
  (bind _charactermovement (Variables|Character|GetCharacterMovement))
  ;[1 1 1] Run
  (:Pressed
    (Variables|/Script/Engine.CharacterMovementComponent|SetMaxWalkSpeed _charactermovement 1e+03)
    (Variables|Default|SetRunning true)
    (CallFunction|DrainStamina))
  (:Released
    (Variables|/Script/Engine.CharacterMovementComponent|SetMaxWalkSpeed _charactermovement 6e+02)
    (Variables|Default|SetRunning false)
    (CallFunction|RefreshStamin)))

(event Input|ActionEvents|InputActionFire
  (params (Key :type Key%20Structure :default "None"))
  (:Pressed
    (bind _asmy_character_bp (Utilities|Casting|CastToMyCharacterBP (Game|GetPlayerCharacter 0)))
    (bind _returnvalue (Class|MyCharacter|GetBulletsinMagazine _asmy_character_bp))
    (if (not (== _returnvalue 0))
      (Class|MyCharacter|Fire _asmy_character_bp)
      (Components|Animation|PlayAnimation (Variables|Default|GetRifleGun) "/Game/Animations/RifleAnimetion/Fire_Pistol_W.Fire_Pistol_W" false))))

(event Input|ActionEvents|InputActionReload
  (params (Key :type Key%20Structure :default "None"))
  ;[1 1 1] Reload
  (:Pressed
    (bind _asmy_character (Utilities|Casting|CastToMyCharacter (Game|GetPlayerCharacter 0)))
    (Class|MyCharacter|ReloadWeapon _asmy_character)))

(event Input|ActionEvents|InputActionSaveGame
  (params (Key :type Key%20Structure :default "None"))
  (:Pressed
    (bind _asmy_shooterok_game_mode_base_bp (Utilities|Casting|CastToMyShooterokGameModeBaseBP (Game|GetGameMode)))
    (Default|SaveGame _asmy_shooterok_game_mode_base_bp)
    (Development|PrintString "Game Saved !")))

(event Input|ActionEvents|InputActionPauseGame
  (params (Key :type Key%20Structure :default "None"))
  (bind _returnvalue (Game|GetPlayerController 0))
  ;[1 1 1] Pause
  (:Pressed
    (Utilities|IsValid (Variables|Default|GetPause%20Menu%20Reference)
      (:Is%20Valid
        _)
      (:Is%20Not%20Valid
        (bind _returnvalue_2 (UserInterface|CreateWidget "/Game/BluePrints/Widgets/PauseWidget.PauseWidget_C"))
        (Variables|Default|SetPause%20Menu%20Reference _returnvalue_2)))
    (Variables|/Script/Engine.PlayerController|SetbShowMouseCursor _returnvalue true)
    (Input|SetInputModeUIOnly _returnvalue (Variables|Default|GetPause%20Menu%20Reference) "DoNotLock")
    (UserInterface|Viewport|AddtoViewport (Variables|Default|GetPause%20Menu%20Reference) 0)
    (Game|SetGamePaused true)))

(event Input|ActionEvents|InputActionLoadGame
  (params (Key :type Key%20Structure :default "None"))
  (:Pressed
    (bind _asmy_shooterok_game_mode_base_bp (Utilities|Casting|CastToMyShooterokGameModeBaseBP (Game|GetGameMode)))
    (Default|LoadSavedData _asmy_shooterok_game_mode_base_bp)
    (Development|PrintString "Game Loaded")))

(event Input|ActionEvents|InputActionReload
  (params (Key :type Key%20Structure :default "None"))
  (:Pressed
    (bind _asmy_character_bp (Utilities|Casting|CastToMyCharacterBP (Game|GetPlayerCharacter 0)))
    (bind _returnvalue (Class|MyCharacter|GetBulletsinMagazine _asmy_character_bp))
    (if (not (== _returnvalue 0))
      (Class|MyCharacter|ReloadWeapon _asmy_character_bp)
      (Variables|Default|SetisReload true))))

(fn ConstructionScript)

(fn InitWeapon
  (bind _asmy_game_settings (Utilities|Casting|CastToMyGameSettings (Game|GetGameInstance)))
  (switch int (Variables|/Game/BluePrints/MyGameSettings.MyGameSettings_C|GetIDCurrentWeapon _asmy_game_settings)
    (:0
      (Components|StaticMesh|SetStaticMesh (Variables|Default|GetFPSGun) "/Game/Meshes/PistolStaticMesh.PistolStaticMesh")
      (Class|SkinnedMeshComponent|SetSkeletalMesh (Variables|Default|GetRifleGun) "/Game/MilitaryWeapDark/Weapons/Pistols_B.Pistols_B" true))
    (:1
      (Components|StaticMesh|SetStaticMesh (Variables|Default|GetFPSGun) "/Game/Meshes/RifleStaticMesh.RifleStaticMesh")
      (Class|SkinnedMeshComponent|SetSkeletalMesh (Variables|Default|GetRifleGun) "/Game/MilitaryWeapDark/Weapons/Assault_Rifle_B.Assault_Rifle_B" true))
    (:2
      (Components|StaticMesh|SetStaticMesh (Variables|Default|GetFPSGun) "/Game/Meshes/ShotgunStaticMesh.ShotgunStaticMesh")
      (Class|SkinnedMeshComponent|SetSkeletalMesh (Variables|Default|GetRifleGun) "/Game/MilitaryWeapDark/Weapons/Shotgun_B.Shotgun_B" true))
    (:3
      (Components|StaticMesh|SetStaticMesh (Variables|Default|GetFPSGun) "/Game/MilitaryWeapDark/Weapons/GrenadeStaticMesh.GrenadeStaticMesh")
      (Class|SkinnedMeshComponent|SetSkeletalMesh (Variables|Default|GetRifleGun) "/Game/MilitaryWeapDark/Weapons/Grenade_Launcher_B.Grenade_Launcher_B" true))))