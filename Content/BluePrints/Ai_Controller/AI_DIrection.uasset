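; AI controller that wanders its pawn around, steering away from obstacles at random.
; Each Tick it traces the Visibility channel ahead along the pawn's forward vector, with a one-frame debug draw.
; A hit rotates the stored Direction by a small yaw step, left or right chosen at random on every hit frame.
; The pawn always receives scaled-down movement input along Direction, whether or not the trace hits.
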(event EventBeginPlay)

(event EventTick
  (params (DeltaSeconds :type Float%20%28single-precision%29))
  (bind _returnvalue (Pawn|GetControlledPawn))
  (bind _returnvalue_2 (Transformation|GetActorLocation _returnvalue))
  (bind _returnvalue_3 (Collision|LineTraceByChannel _returnvalue_2 (+ _returnvalue_2 (* (Transformation|GetActorForwardVector _returnvalue) 1000)) "TraceTypeQuery1" false 0 "ForOneFrame"))
  (if _returnvalue_3
    ;[1 1 1] Random change direcrion when we see the prevention
    (Variables|Default|SetRandomDirection (Math|Conversions|ToFloat(Integer) (Math|Integer|SelectInt 10 -10 (Math|Random|RandomBool))))
    (Variables|Default|SetDirection (Math|Vector|RotateVector (Variables|Default|GetDirection) (Math|Rotator|MakeRotator 0.0 0.0 (Variables|Default|GetRandomDirection)))))
  (Pawn|Input|AddMovementInput _returnvalue (Variables|Default|GetDirection) 0.3 false))

(fn ConstructionScript)