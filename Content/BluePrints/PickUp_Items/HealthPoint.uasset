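; Health pickup actor that spins, moves vertically and heals the player character on contact.
; A timeline started on BeginPlay drives the root's yaw and height, adding a third of the owner's Z when an owner is valid.
; Sphere overlap with MyCharacterBP, only when truncated Health is below truncated FullHealth, calls PickUpHp, destroys the pickup and plays a sound at its location.
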(event OnComponentBeginOverlap(Sphere)
  (params (OverlappedComponent :type Primitive%20Component%20Object%20Reference) (OtherActor :type Actor%20Object%20Reference) (OtherComp :type Primitive%20Component%20Object%20Reference) (OtherBodyIndex :type Integer) (bFromSweep :type Boolean) (SweepResult :type Hit%20Result%20Structure%20%28by%20ref%29))
  ;[1 1 1] Pick Up
  (bind _asmy_character_bp (Utilities|Casting|CastToMyCharacterBP OtherActor))
  (if (not (>= (Math|Float|Truncate (Variables|/Script/Shooterok.MyCharacter|GetHealth _asmy_character_bp)) (Math|Float|Truncate (Variables|/Script/Shooterok.MyCharacter|GetFullHealth _asmy_character_bp))))
    (Class|MyCharacter|PickUpHp _asmy_character_bp)
    (Actor|DestroyActor)
    (Audio|SpawnSoundatLocation "/Game/Sounds/health-pickup-6860_Cue.health-pickup-6860_Cue" (Transformation|GetActorLocation) "0, 0, 0" 1.0 1.0 0.0 0 0)))

(event OnComponentEndOverlap(Sphere)
  (params (OverlappedComponent :type Primitive%20Component%20Object%20Reference) (OtherActor :type Actor%20Object%20Reference) (OtherComp :type Primitive%20Component%20Object%20Reference) (OtherBodyIndex :type Integer)))

(event EventBeginPlay
  (bind _returnvalue (Components|GetOwner))
  (bind _returnvalue_2 (Transformation|GetActorLocation))
  (bind _defaultsceneroot (Variables|Default|GetDefaultSceneRoot))
  ;[1 1 1] Animation
  (bind (_direction _rotation _newtrack_0) (Timeline|Timeline_0 Play)
    (:Update
      (Transformation|SetRelativeRotation _defaultsceneroot (Math|Rotator|MakeRotator 0.0 0.0 _rotation) false false)
      (Utilities|IsValid _returnvalue
        (:Is%20Valid
          (Transformation|SetRelativeLocation _defaultsceneroot (Math|Vector|MakeVector (.x _returnvalue_2) (.y _returnvalue_2) (+ (/ (.z (Transformation|GetActorLocation _returnvalue)) 3.0) _newtrack_0)) false false))
        (:Is%20Not%20Valid
          (Transformation|SetRelativeLocation _defaultsceneroot (Math|Vector|MakeVector (.x _returnvalue_2) (.y _returnvalue_2) _newtrack_0) false false))))))

(fn ConstructionScript)