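; Rifle ammo pickup actor that refills the player's bullets on overlap.
; A timeline started at BeginPlay animates the static mesh's yaw and height as an idle pickup effect.
; Sphere overlap casts to MyCharacterBP and, only if its bullet count is below the maximum, calls PickUpAmmo and destroys the pickup.
; NewFunction0, which moves the actor to the world origin, is not called within this Blueprint.
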(event OnComponentBeginOverlap(Sphere)
  (params (OverlappedComponent :type Primitive%20Component%20Object%20Reference) (OtherActor :type Actor%20Object%20Reference) (OtherComp :type Primitive%20Component%20Object%20Reference) (OtherBodyIndex :type Integer) (bFromSweep :type Boolean) (SweepResult :type Hit%20Result%20Structure%20%28by%20ref%29))
  ;[1 1 1] Pick Up
  (bind _asmy_character_bp (Utilities|Casting|CastToMyCharacterBP OtherActor))
  (bind _returnvalue (Class|MyCharacter|GetCountBullets _asmy_character_bp))
  (if (< _returnvalue (Class|MyCharacter|GetMaxCountBullets _asmy_character_bp))
    (Class|MyCharacter|PickUpAmmo _asmy_character_bp)
    (Actor|DestroyActor)))

(event EventBeginPlay
  (bind _staticmesh (Variables|Default|GetStaticMesh))
  ;[1 1 1] Animation
  (bind (_direction _rotation _newtrack_0) (Timeline|Move Play)
    (:Update
      (Transformation|SetRelativeRotation _staticmesh (Math|Rotator|MakeRotator 0.0 0.0 _rotation) false false)
      (Transformation|SetRelativeLocation _staticmesh (Math|Vector|MakeVector 0.0 0.0 _newtrack_0) false false))))

(fn ConstructionScript)

(fn NewFunction0
  (Transformation|SetActorLocation "0, 0, 0" false false))