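; MyGameSettings is a Game Instance Blueprint that manages the player's weapon list, level-gated inventory and equipped weapon.
; InitWeaponList loads WeaponList from a DataTable, and InitInventoryList copies entries at or below Level into WeaponInventoryList, flagging IDCurrentWeapon as equipped.
; SetEquipedWeapon rewrites WeaponList flags by ID.
; RefreshInventoryList wraps WeaponList, not the filtered list, in UWeaponData objects for the list view; SaveGame is an empty stub.
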(fn SaveGame)

(fn RefreshInventoryList
  (bind _inventoryweaponlist (Variables|Default|GetInventoryWeaponList))
  (Class|ListView|ClearListItems _inventoryweaponlist)
  (for _array_element (Variables|Default|GetWeaponList)
    (bind _returnvalue (Game|ConstructObjectfromClass "/Game/BluePrints/Widgets/Data/UWeaponData.UWeaponData_C" self))
    (Variables|/Game/BluePrints/Widgets/Data/UWeaponData.UWeaponData_C|SetData _returnvalue _array_element)
    (Class|ListView|AddItem _inventoryweaponlist _returnvalue)))

(fn InitWeaponList
  (Utilities|Array|Clear (Variables|Default|GetWeaponList))
  (bind _outrownames (DataTable|GetDataTableRowNames "/Game/BluePrints/Widgets/Data/WeaponsDataTable.WeaponsDataTable"))
  (for _array_element _outrownames
    (bind _returnvalue (Utilities|GetDataTableRow "/Game/BluePrints/Widgets/Data/WeaponsDataTable.WeaponsDataTable" _array_element)
      (:then
        (Utilities|Array|Add (Variables|Default|GetWeaponList) _returnvalue)))))

(fn SetEquipedWeapon
  (params (IdWeaponEquiped :type Integer))
  (bind _weaponlist (Variables|Default|GetWeaponList))
  (for (_array_element _array_index) _weaponlist
    (if (== (.id _array_element) IdWeaponEquiped)
      (Utilities|Array|SetArrayElem _weaponlist _array_index (Utilities|Struct|MakeSDataWeapon (.id _array_element) (.image _array_element) (.name _array_element) (.damage _array_element) (.rateoffire _array_element) (.level _array_element) true true))
      (else
        (Utilities|Array|SetArrayElem _weaponlist _array_index (Utilities|Struct|MakeSDataWeapon (.id _array_element) (.image _array_element) (.name _array_element) (.damage _array_element) (.rateoffire _array_element) (.level _array_element) false true))))))

(fn InitInventoryList
  (bind _weaponlist (Variables|Default|GetWeaponList))
  (bind _weaponinventorylist (Variables|Default|GetWeaponInventoryList))
  (Utilities|Array|Clear _weaponlist)
  (CallFunction|InitWeaponList)
  (Utilities|Array|Clear _weaponinventorylist)
  (bind _asmy_game_settings (Utilities|Casting|CastToMyGameSettings (Game|GetGameInstance)))
  (for _array_element _weaponlist
    (if (>= (Variables|Default|GetLevel) (.Level (Utilities|Struct|BreakSDataWeapon _array_element)))
      (if (== (Variables|MyGameSettings_C|GetIDCurrentWeapon _asmy_game_settings) (.Id (Utilities|Struct|BreakSDataWeapon _array_element)))
        (Utilities|Array|Add _weaponinventorylist (Utilities|Struct|MakeSDataWeapon (.Id (Utilities|Struct|BreakSDataWeapon _array_element)) (.Image (Utilities|Struct|BreakSDataWeapon _array_element)) (.Name (Utilities|Struct|BreakSDataWeapon _array_element)) (.Damage (Utilities|Struct|BreakSDataWeapon _array_element)) (.Rateoffire (Utilities|Struct|BreakSDataWeapon _array_element)) (.Level (Utilities|Struct|BreakSDataWeapon _array_element)) true true))
        (else
          (Utilities|Array|Add _weaponinventorylist (Utilities|Struct|MakeSDataWeapon (.Id (Utilities|Struct|BreakSDataWeapon _array_element)) (.Image (Utilities|Struct|BreakSDataWeapon _array_element)) (.Name (Utilities|Struct|BreakSDataWeapon _array_element)) (.Damage (Utilities|Struct|BreakSDataWeapon _array_element)) (.Rateoffire (Utilities|Struct|BreakSDataWeapon _array_element)) (.Level (Utilities|Struct|BreakSDataWeapon _array_element)) false true)))))))