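; Shooter game mode that owns saving, loading and restarting through the single "save1" slot.
; BeginPlay creates that save or applies it to MyCharacterBP (transform, stats, settings), also copying level to MyGameSettings.
; Saved ammo and weapon ID are restored only when that ID differs from MyGameSettings' current weapon.
; SaveGame writes character state back; LoadGame reloads the map to re-trigger loading, while RestartLevel deletes the save first.
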(event Custom|Save%20Game
  (bind _returnvalue (Game|GetPlayerCharacter 0))
  ;[1 1 1] Save Game
  (bind _returnvalue_2 (SaveGame|LoadGamefromSlot "save1"))
  (bind _asshooter_save_game (Utilities|Casting|CastToShooterSaveGame _returnvalue_2))
  (bind _asmy_character_bp (Utilities|Casting|CastToMyCharacterBP _returnvalue))
  (Utilities|FlowControl|Sequence
    (:then_0
      (Variables|/Game/BluePrints/ShooterSaveGame.ShooterSaveGame_C|SetHero%20Transform _asshooter_save_game (Transformation|GetActorTransform _returnvalue)))
    (:then_1
      (Variables|/Game/BluePrints/ShooterSaveGame.ShooterSaveGame_C|SetExpirience _asshooter_save_game (Variables|/Script/Shooterok.MyCharacter|GetExpirience _asmy_character_bp)))
    (:then_2
      (Variables|/Game/BluePrints/ShooterSaveGame.ShooterSaveGame_C|SetbaseTurnRate _asshooter_save_game (Variables|/Script/Shooterok.MyCharacter|GetBaseTurnRate _asmy_character_bp)))
    (:then_3
      (Variables|/Game/BluePrints/ShooterSaveGame.ShooterSaveGame_C|SetbaseUpRate _asshooter_save_game (Variables|/Script/Shooterok.MyCharacter|GetBaseLookUpRate _asmy_character_bp)))
    (:then_4
      (Variables|/Game/BluePrints/ShooterSaveGame.ShooterSaveGame_C|Setkills _asshooter_save_game (Variables|/Script/Shooterok.MyCharacter|GetKills _asmy_character_bp)))
    (:then_5
      (Variables|/Game/BluePrints/ShooterSaveGame.ShooterSaveGame_C|SetbaseVolume _asshooter_save_game (Variables|/Script/Shooterok.MyCharacter|GetBaseVolume _asmy_character_bp)))
    (:then_6
      (bind _returnvalue_3 (Class|MyCharacter|GetCountBullets _asmy_character_bp))
      (Variables|/Game/BluePrints/ShooterSaveGame.ShooterSaveGame_C|Setbullet%20count _asshooter_save_game _returnvalue_3))
    (:then_7
      (bind _returnvalue_4 (Class|MyCharacter|GetBulletsinMagazine _asmy_character_bp))
      (Variables|/Game/BluePrints/ShooterSaveGame.ShooterSaveGame_C|Setbullet%20in%20magazine%20count _asshooter_save_game _returnvalue_4))
    (:then_8
      (Variables|/Game/BluePrints/ShooterSaveGame.ShooterSaveGame_C|SetLevel _asshooter_save_game (Variables|/Script/Shooterok.MyCharacter|GetLevel _asmy_character_bp)))
    (:then_9
      (Variables|/Game/BluePrints/ShooterSaveGame.ShooterSaveGame_C|SetHealthPoint _asshooter_save_game (Math|Float|Truncate (Variables|/Script/Shooterok.MyCharacter|GetHealth _asmy_character_bp))))
    (:then_10
      (bind _returnvalue_5 (Class|MyCharacter|GetWeaponId _asmy_character_bp))
      (Variables|/Game/BluePrints/ShooterSaveGame.ShooterSaveGame_C|SetIdWeaponFromSaveGame _asshooter_save_game _returnvalue_5))
    (:then_11
      (SaveGame|SaveGametoSlot _asshooter_save_game "save1"))))

(event Custom|Load%20Game
  (Development|ExecuteConsoleCommand "RestartLevel" 0))

(event Custom|RestartLevel
  (SaveGame|DeleteGameinSlot "save1")
  (Development|ExecuteConsoleCommand "RestartLevel" 0))

(event Custom|LoadSavedData
  (bind _returnvalue (Game|GetPlayerCharacter 0))
  ;[1 1 1] Load Data
  (bind _returnvalue_2 (SaveGame|LoadGamefromSlot "save1"))
  (bind _asshooter_save_game (Utilities|Casting|CastToShooterSaveGame _returnvalue_2))
  (bind _asmy_character_bp (Utilities|Casting|CastToMyCharacterBP _returnvalue))
  (Utilities|FlowControl|Sequence
    (:then_0
      (Transformation|SetWorldTransform (Variables|/Script/Engine.Actor|GetRootComponent _returnvalue) (Variables|/Game/BluePrints/ShooterSaveGame.ShooterSaveGame_C|GetHero%20Transform _asshooter_save_game) false false))
    (:then_1
      (Class|MyCharacter|SetBaseTurnRate _asmy_character_bp (Variables|/Game/BluePrints/ShooterSaveGame.ShooterSaveGame_C|GetbaseTurnRate _asshooter_save_game)))
    (:then_2
      (Class|MyCharacter|SetBaseUpRate _asmy_character_bp (Variables|/Game/BluePrints/ShooterSaveGame.ShooterSaveGame_C|GetbaseUpRate _asshooter_save_game)))
    (:then_3
      (Variables|/Script/Shooterok.MyCharacter|SetBaseVolume _asmy_character_bp (Variables|/Game/BluePrints/ShooterSaveGame.ShooterSaveGame_C|GetbaseVolume _asshooter_save_game)))
    (:then_4
      (Variables|/Script/Shooterok.MyCharacter|SetExpirience _asmy_character_bp (Variables|/Game/BluePrints/ShooterSaveGame.ShooterSaveGame_C|GetExpirience _asshooter_save_game)))
    (:then_5
      (Variables|/Script/Shooterok.MyCharacter|SetHealth _asmy_character_bp (Math|Conversions|ToFloat(Integer) (Variables|/Game/BluePrints/ShooterSaveGame.ShooterSaveGame_C|GetHealthPoint _asshooter_save_game))))
    (:then_6
      (Variables|/Script/Shooterok.MyCharacter|SetKills _asmy_character_bp (Variables|/Game/BluePrints/ShooterSaveGame.ShooterSaveGame_C|Getkills _asshooter_save_game)))
    (:then_7
      (Variables|/Script/Shooterok.MyCharacter|SetLevel _asmy_character_bp (Variables|/Game/BluePrints/ShooterSaveGame.ShooterSaveGame_C|GetLevel _asshooter_save_game)))
    (:then_8
      (bind _asmy_game_settings (Utilities|Casting|CastToMyGameSettings (Game|GetGameInstance)))
      (Variables|/Game/BluePrints/MyGameSettings.MyGameSettings_C|SetLevel _asmy_game_settings (Variables|/Game/BluePrints/ShooterSaveGame.ShooterSaveGame_C|GetLevel _asshooter_save_game)))
    (:then_9
      (CallFunction|LoadWeaponSettings _asshooter_save_game))))

(event EventBeginPlay
  (bind _returnvalue (SaveGame|DoesSaveGameExist "save1"))
  (if _returnvalue
    (CallFunction|LoadSavedData)
    (else
      ;[1 1 1] Create Save file
      (bind _returnvalue_2 (SaveGame|CreateSaveGameObject "/Game/BluePrints/ShooterSaveGame.ShooterSaveGame_C"))
      (SaveGame|SaveGametoSlot _returnvalue_2 "save1"))))

(fn ConstructionScript)

(fn IfWeaponChanged
  (params (IdNewWeapon :type Integer))
  (bind _asmy_game_settings (Utilities|Casting|CastToMyGameSettings (Game|GetGameInstance)))
  (return (!= (Variables|/Game/BluePrints/MyGameSettings.MyGameSettings_C|GetIDCurrentWeapon _asmy_game_settings) IdNewWeapon)))

(fn LoadWeaponSettings
  (params (Save%20obj :type Shooter%20Save%20Game%20Object%20Reference))
  (bind _idweaponfromsavegame (Variables|/Game/BluePrints/ShooterSaveGame.ShooterSaveGame_C|GetIdWeaponFromSaveGame Save%20obj))
  (bind _asmy_character_bp (Utilities|Casting|CastToMyCharacterBP (Game|GetPlayerCharacter 0)))
  (bind _ifchanged (CallFunction|IfWeaponChanged _idweaponfromsavegame))
  (if _ifchanged
    (Utilities|FlowControl|Sequence
      (:then_0
        (Class|MyCharacter|SetCountBullets _asmy_character_bp (Variables|/Game/BluePrints/ShooterSaveGame.ShooterSaveGame_C|Getbullet%20count Save%20obj)))
      (:then_1
        (Class|MyCharacter|SetBulletsinMagazine _asmy_character_bp (Variables|/Game/BluePrints/ShooterSaveGame.ShooterSaveGame_C|Getbullet%20in%20magazine%20count Save%20obj)))
      (:then_2
        (bind _asmy_game_settings (Utilities|Casting|CastToMyGameSettings (Game|GetGameInstance)))
        (Variables|/Game/BluePrints/MyGameSettings.MyGameSettings_C|SetIDCurrentWeapon _asmy_game_settings _idweaponfromsavegame)))))